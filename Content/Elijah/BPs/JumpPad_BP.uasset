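; Jump pad actor that launches an overlapping Parkourer along its Arrow component's forward vector, scaled by JumpPadStrength.
; The box overlap triggers the launch, which adds to the character's existing velocity rather than overriding it.
; After short delays, MoveComponentTo tilts the pad base and eases it back as a spring animation.
; An unconnected SetActorRotation node for turning the character toward the launch is never executed.
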(event `self.Box.OnComponentBeginOverlap`
  (params (OverlappedComponent :type "PrimitiveComponent Object Reference") (OtherActor :type "Actor Object Reference") (OtherComp :type "PrimitiveComponent Object Reference") (OtherBodyIndex :type Integer) (bFromSweep :type Boolean) (SweepResult :type "HitResult Structure (by ref)"))
  (bind _jumppadbase (`self.JumpPadBase`))
  (bind _asparkourer (cast `/Game/Elijah/BPs/Parkourer` OtherActor))
  (`Character.LaunchCharacter` _asparkourer (* (`SceneComponent.GetForwardVector` (`self.Arrow`)) (`self.JumpPad Strength`)) false false)
  (`KismetSystemLibrary.Delay` 0.1)
  (`KismetSystemLibrary.MoveComponentTo` _jumppadbase (0.0 0.0 0.0) (struct :`Roll` -90.0) false true)
  (`KismetSystemLibrary.Delay` 0.01)
  (`KismetSystemLibrary.MoveComponentTo` _jumppadbase (0.0 0.0 0.0) (struct) false true))

(fn `UserConstructionScript`)